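; Player character "julian" with movement, camera look and picking up and dropping of physics objects.
; Movement follows control yaw, while the VistaUP axis drives yaw and VistaRight drives pitch.
; The "coger" input toggles between releasing and grabbing, using a 500-unit camera line trace to find a simulating component.
; A PhysicsHandle holds the grabbed component, its target updated every Tick to the "Loc.objeto" position.
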(event `self.ReceiveTick`
  (params (DeltaSeconds :type "Float (single-precision)"))
  ;[1 1 1] evento marcar
  (`|ExecutionSequence`
    (:`then_0`
      ;[1 1 1] Coger Soltar objeto
      (`PhysicsHandleComponent.SetTargetLocation` (`self.PhysicsHandle`) (`SceneComponent.K2_GetComponentLocation` (`self.loc.objeto`))))))

(event `soltar objeto`
  ;[1 1 1] Coger Soltar objeto
  (`PhysicsHandleComponent.ReleaseComponent` (`self.PhysicsHandle`))
  (set `self.estacogiendoobjeto?` false))

(event `InputAction|coger`
  (params (Key :type "Key Structure"))
  ;[1 1 1] Coger Soltar objeto
  (:`Pressed`
    (if (`self.estacogiendoobjeto?`)
      (`self.soltar objeto`)
      (else
        (`self.coger Objeto`)))))

(event `coger Objeto`
  (bind _returnvalue (`GameplayStatics.GetPlayerCameraManager` 0))
  (bind _returnvalue_2 (`self.K2_GetActorLocation` _returnvalue))
  ;[1 1 1] Coger Soltar objeto
  (bind _outhit (`KismetSystemLibrary.LineTraceSingle` _returnvalue_2 (+ (* (`self.GetActorForwardVector` _returnvalue) 500) _returnvalue_2) "TraceTypeQuery1"))
  (if true
    (bind (_bblockinghit _binitialoverlap _time _distance _location _impactpoint _normal _impactnormal _physmat _hitactor _hitcomponent) (`GameplayStatics.BreakHitResult` _outhit))
    (if (`SceneComponent.IsSimulatingPhysics` _hitcomponent "None")
      (`PhysicsHandleComponent.GrabComponentAtLocation` (`self.PhysicsHandle`) _hitcomponent "None" (`SceneComponent.K2_GetComponentLocation` _hitcomponent))
      (set `self.estacogiendoobjeto?` true))))

(event `InputAxis|MoveRight`
  (params (AxisValue :type "Float (single-precision)"))
  (bind (_returnvalue_roll _returnvalue_pitch _returnvalue_yaw) (`KismetMathLibrary.BreakRotator` (`self.GetControlRotation`)))
  ;[1 1 1] Movimiento camara y personaje
  (`self.AddMovementInput` (`KismetMathLibrary.GetRightVector` (`KismetMathLibrary.MakeRotator` 0.0 0.0 _returnvalue_yaw)) AxisValue))

(event `InputAxis|MoveForward`
  (params (AxisValue :type "Float (single-precision)"))
  (bind (_returnvalue_roll _returnvalue_pitch _returnvalue_yaw) (`KismetMathLibrary.BreakRotator` (`self.GetControlRotation`)))
  ;[1 1 1] Movimiento camara y personaje
  (`self.AddMovementInput` (`KismetMathLibrary.GetForwardVector` (`KismetMathLibrary.MakeRotator` 0.0 0.0 _returnvalue_yaw)) AxisValue))

(event `InputAxis|VistaUP`
  (params (AxisValue :type "Float (single-precision)"))
  ;[1 1 1] Movimiento camara y personaje
  (`self.AddControllerYawInput` AxisValue))

(event `InputAxis|VistaRight`
  (params (AxisValue :type "Float (single-precision)"))
  ;[1 1 1] Movimiento camara y personaje
  (`self.AddControllerPitchInput` AxisValue))

(fn `UserConstructionScript`)